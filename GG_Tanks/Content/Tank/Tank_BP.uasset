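; Player tank Blueprint that sets up turret and barrel references and handles camera-style aim input.
; On BeginPlay it passes the Turret and Barrel components to the SetTurretReference and SetBarrelReference functions.
; AimAzimuth yaws the Scene component and AimAltitude pitches the SpringArm, both scaled by frame delta time with separate speeds.
; The graphs rotate only these two components, never the turret or barrel directly.
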(event `self.ReceiveBeginPlay`
  (`self.SetTurretReference` (`self.Turret`))
  (`self.SetBarrelReference` (`self.Barrel`)))

(event `InputAxis|AimAzimuth`
  (params (AxisValue :type "Float (single-precision)"))
  (`SceneComponent.K2_AddLocalRotation` (`self.Scene`) (`KismetMathLibrary.MakeRotator` 0.0 0.0 (* AxisValue (`GameplayStatics.GetWorldDeltaSeconds`) 100.0)) false false))

(event `InputAxis|AimAltitude`
  (params (AxisValue :type "Float (single-precision)"))
  (`SceneComponent.K2_AddLocalRotation` (`self.SpringArm`) (`KismetMathLibrary.MakeRotator` 0.0 (* AxisValue (`GameplayStatics.GetWorldDeltaSeconds`) 50.0)) false false))

(fn `UserConstructionScript`)